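; FPS player state Blueprint that tracks ammo per weapon type in an AmmoData map of structs holding current clip and reserve counts.
; BI-prefixed events consume, set, add and reload ammo by looking up the weapon's entry and setting its struct members.
; Reload fills the clip from the reserve and returns unused rounds to it, while BICanReload checks for a non-full clip and remaining reserve.
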(event EventBIConsumeClipAmmo
  (params (weaponType :type EWeaponType%20Enum :default "NewEnumerator2"))
  (bind _ammodata (Variables|Default|GetAmmoData))
  (bind (_value _returnvalue) (Utilities|Map|Find _ammodata weaponType))
  ;[1 0.4791 0.489] Consume ammo from clip
  (if _returnvalue
    (bind _result (Math|Integer|DecrementInt (.CurrentAmmo (Utilities|Struct|BreakAmmoDataStruct _value)))
      (:%20%20
        (Utilities|Struct|SetmembersinAmmoDataStruct _value _result)))))

(event EventBISetAmmoData
  (params (weaponType :type EWeaponType%20Enum :default "NewEnumerator2") (ammoData :type Ammo%20Data%20Struct%20Structure))
  (bind _ammodata (Variables|Default|GetAmmoData))
  (bind (_value _returnvalue) (Utilities|Map|Find _ammodata weaponType))
  ;[0.9909 1 0.6084] Set ammo data
  (if _returnvalue
    (Utilities|Struct|SetmembersinAmmoDataStruct _value (.currentammo ammoData) (.totalammoleft ammoData))))

(event EventBIAddAmmo
  (params (weaponType :type EWeaponType%20Enum :default "NewEnumerator2") (addedAmount :type Integer))
  (bind _ammodata (Variables|Default|GetAmmoData))
  (bind (_value _returnvalue) (Utilities|Map|Find _ammodata weaponType))
  ;[0.4248 1 0.6605] Add total ammo
  (if _returnvalue
    (Utilities|Struct|SetmembersinAmmoDataStruct _value (+ (.TotalAmmoLeft (Utilities|Struct|BreakAmmoDataStruct _value)) addedAmount))))

(event EventBIReloadClip
  (params (weaponType :type EWeaponType%20Enum :default "NewEnumerator2") (clipSize :type Integer))
  (bind _ammodata (Variables|Default|GetAmmoData))
  (bind (_value _returnvalue) (Utilities|Map|Find _ammodata weaponType))
  (bind (_currentammo _totalammoleft) (Utilities|Struct|BreakAmmoDataStruct _value))
  (bind _returnvalue_2 (Math|Integer|Min(Integer) clipSize _totalammoleft))
  ;[0.6151 0.492 1] Reload clip
  (if _returnvalue
    (Variables|Default|SetTempAmmo _currentammo)
    (bind _structout (Utilities|Struct|SetmembersinAmmoDataStruct _value _returnvalue_2))
    (Utilities|Struct|SetmembersinAmmoDataStruct _structout (Math|Integer|Max(Integer) 0 (- (+ (Variables|Default|GetTempAmmo) _totalammoleft) _returnvalue_2)))))

(fn ConstructionScript)

(fn BICanReload
  (params (weaponType :type EWeaponType%20Enum :default "NewEnumerator2") (clipSize :type Integer))
  (bind _ammodata (Variables|Default|GetAmmoData))
  (bind (_value _returnvalue) (Utilities|Map|Find _ammodata weaponType))
  (bind (_currentammo _totalammoleft) (Utilities|Struct|BreakAmmoDataStruct _value))
  (if _returnvalue
    (return (and (< _currentammo clipSize) (> _totalammoleft 0)))
    (else
      (return false))))