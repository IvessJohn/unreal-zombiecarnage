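; Game mode for a wave-based zombie survival level that alternates timed intermissions with waves until the last one is cleared.
; Spawn and kill events update per-wave counters, switching tagged BP_ZombieSpawner actors on or off to respect each wave's size and an optional alive cap.
; Wave, intermission and level-end changes are messaged to the player controller, with sounds for key moments.
; A separate LevelFailed event handles defeat, and stat getters expose progress.
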(event EventBeginPlay
  ;[0.8848 0.7498 1] BeginPlay
  (CallFunction|LevelStart))

(event EventLevelComplete
  ;[0.4536 1 0.3115] Level Complete
  (CallFunction|LevelEnd)
  (Audio|PlaySound2D 0 1.0 1.0 0.0 0 0)
  (Class|BPIGameplayFramework|LevelComplete(Message) (Game|GetPlayerController 0)))

(event EventWaveStarted
  ;[0.5955 0.9198 1] Start wave
  (CallFunction|StartWave)
  (Class|BPIGameplayFramework|WaveStarted(Message) (Game|GetPlayerController 0)))

(event EventZombieSpawned
  (params (ZombieRef :type BP%20Enemy%20Object%20Reference))
  ;[1 0.6605 0.519] Zombie spawned
  (Utilities|FlowControl|Sequence
    (:then_0
      (Math|Integer|IncrementInt (Variables|Zombies|GetZombiesSpawnedOnThisWave)))
    (:then_1
      (Math|Integer|IncrementInt (Variables|Zombies|GetZombiesAlive)
        (:%20%20
          (if (CallFunction|HasZombiesReachedtheAliveLimit?)
            (CallFunction|ProhibitSpawningEnemies :!label _label)))))
    (:then_2
      (Math|Integer|DecrementInt (Variables|Zombies|GetZombiesLeftToSpawn)
        (:%20%20
          (if (not (Utilities|AnyZombiesLefttoSpawn?))
            (goto _label)))))))

(event EventZombieKilled
  ;[0.8638 1 0.8509] Zombie died
  (Math|Integer|DecrementInt (Variables|Zombies|GetZombiesAlive)
    (:%20%20
      (Math|Integer|IncrementInt (Variables|Zombies|GetZombiesKilledOnThisWave)
        (:%20%20
          (if (Utilities|AnyZombiesLefttoKill?)
            (if (Utilities|AnyZombiesLefttoSpawn?)
              (CallFunction|AllowSpawningEnemies))
            (else
              (CallFunction|WaveEnded))))))))

(event EventWaveEnded
  ;[0.5637 1 0.5878] Wave Ended
  (Utilities|FlowControl|Sequence
    (:then_0
      (Development|PrintString "Wave completed!")
      (CallFunction|ProhibitSpawningEnemies)
      (Audio|PlaySound2D 0 1.0 1.0 0.0 0 0) ; Play wave end sound
    )
    (:then_1
      (Class|BPIGameplayFramework|WaveEnded(Message) (Game|GetPlayerController 0)))
    (:then_2
      (if (Utilities|IsIttheLastWave?)
        (CallFunction|LevelComplete)
        (else
          (CallFunction|StartIntermission))))))

(event EventLevelStart
  ;[0.8417 0.6237 1] Level Start
  (CallFunction|StartIntermission))

(event EventLevelFailed
  ;[1 0.4389 0.3591] Level Failed
  (CallFunction|LevelEnd)
  (Audio|PlaySound2D "/Game/_Main/SFX/Other/GameLost.GameLost" 1.0 1.0 0.0 0 0)
  (Class|BPIGameplayFramework|LevelFailed(Message) (Game|GetPlayerController 0)))

(event EventLevelEnd
  ;[0.9982 0.5801 1] Level End
  (Class|BPIGameplayFramework|LevelEnd(Message) (Game|GetPlayerController 0)))

(fn ConstructionScript)

(fn GetZombiesonThisWave
  (return (Utilities|Array|Get(acopy) (Variables|Game|GetZombiesOnWaves) (Variables|Game|GetCurrentWaveId))))

(fn GetTotalWaves
  (return (+ (CallFunction|GetLastWaveIndex) 1)))

(fn AllowSpawningEnemies
  (Development|PrintString "Allow zombie spawning")
  (Variables|Zombies|SetcanSpawnZombies? true)
  (bind _outactors (Actor|GetAllActorsOfClasswithTag "/Game/_Main/Blueprints/Enemies/BP_ZombieSpawner.BP_ZombieSpawner_C" "ZombieSpawner"))
  (bind _array_element (Utilities|Array|ForEachLoopwithBreak _outactors)
    (:LoopBody
      (Class|BPIZombieSpawner|StartZombieSpawning(Message) _array_element))))

(fn StartIntermission
  (Utilities|FlowControl|Sequence
    (:then_0
      (Utilities|Time|SetTimerbyFunctionName 0 "EndIntermission" (CallFunction|GetIntermissionDurationforWave (Variables|Game|GetCurrentWaveId))))
    (:then_1
      (Class|BPIGameplayFramework|IntermissionStarted(Message) (Game|GetPlayerController 0)))))

(fn EndIntermission
  (CallFunction|WaveStarted))

(fn ProhibitSpawningEnemies
  (Development|PrintString "Prohibit zombie spawning")
  (Variables|Zombies|SetcanSpawnZombies? false)
  (bind _outactors (Actor|GetAllActorsOfClasswithTag "/Game/_Main/Blueprints/Enemies/BP_ZombieSpawner.BP_ZombieSpawner_C" "ZombieSpawner"))
  (bind _array_element (Utilities|Array|ForEachLoopwithBreak _outactors)
    (:LoopBody
      (Variables|/Game/_Main/Blueprints/Enemies/BP_ZombieSpawner.BP_ZombieSpawner_C|SetcanSpawn? _array_element false))))

(fn StartWave
  (Utilities|FlowControl|Sequence
    (:then_0
      (Variables|Zombies|SetZombiesSpawnedOnThisWave 0)
      (Variables|Zombies|SetZombiesKilledOnThisWave 0))
    (:then_1
      (Math|Integer|IncrementInt (Variables|Game|GetCurrentWaveId)
        (:%20%20
          (Variables|Zombies|SetZombiesLeftToSpawn (CallFunction|GetZombiesonThisWave))
          (CallFunction|AllowSpawningEnemies)
          (Audio|PlaySound2D 0 1.0 1.0 0.0 0 0) ; Play wave start sound
        )))
    (:then_2
      (Audio|PlaySound2D "/Game/_Main/SFX/Other/WaveStart_1.WaveStart_1" 0.9 1.0 0.0 0 0))
    (:then_3
      (Development|PrintString "Wave started!"))))

(fn HasZombiesReachedtheAliveLimit?
  (if (<= (Variables|Zombies|GetMaxZombiesAlive) 0)
    (return false) ; If the limit is set to 0, then the number of zombies alive is unlimited
    (else
      (return (>= (Variables|Zombies|GetZombiesAlive) (Variables|Zombies|GetMaxZombiesAlive))))))

(fn GetZombiesLefttoKill
  (return (- (CallFunction|GetZombiesonThisWave) (Variables|Zombies|GetZombiesKilledOnThisWave))))

(fn GetLastWaveIndex
  (if (> (Variables|Game|GetWavesToSurvive) 0)
    (return (- (Variables|Game|GetWavesToSurvive) 1))
    (else
      (return (Utilities|Array|LastIndex (Variables|Game|GetZombiesOnWaves))))))

(fn GetIntermissionDurationforWave
  (params (WaveId :type Integer))
  (if (== WaveId -1)
    (return (Variables|Game|GetFirstIntermissionDuration))
    (else
      (return (Variables|Game|GetIntermissionDuration)))))

(fn StatsGetCurrentWave
  (return (Variables|Game|GetCurrentWaveId)))

(fn StatsGetZombiesLefttoKill
  (return (CallFunction|GetZombiesLefttoKill)))