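; Zombie enemy that chases the player, attacking in melee or with thrown projectiles.
; AIMoveTo loops into melee on arrival, while a randomized reload timer attempts throws when a line trace finds the player.
; Montage notifies time the sphere-overlap hit and projectile spawn.
; Sight or damage triggers running, noise can start pursuit, and point damage scales by hit surface until death notifies the game mode and destroys the actor.
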(event OnHearNoise(PawnSensing)
  (params (Instigator :type Pawn%20Object%20Reference) (Location :type Vector%20%28by%20ref%29 :default "0, 0, 0") (Volume :type Float%20%28single-precision%29))
  ;[0.7655 1 0.7134] Hear player noise
  (if (and (== Instigator (Game|GetPlayerController 0)) (not (Variables|Movement|GetisFollowingPlayer?)))
    (CallFunction|FollowPlayer)
    (Variables|/Script/AIModule.PawnSensingComponent|SetbHearNoises (Variables|Default|GetPawnSensing) false)))

(event OnSeePawn(PawnSensing)
  (params (Pawn :type Pawn%20Object%20Reference))
  ;[0.5725 1 0.6935] See player
  (CallFunction|Outrage))

(event Custom|FollowPlayer
  ;[1 1 1] Follow player
  (if (and (not (Variables|Default|GetisDead?)) (Variables|Default|GetisActive?))
    (Pawn|Components|CharacterMovement|SetMovementMode (Variables|Character|GetCharacterMovement) "MOVE_Walking" 0)
    (Variables|Movement|SetisFollowingPlayer? true)
    (AI|AIMoveTo self "0, 0, 0" (Game|Player|GetPlayerPawn 0) 3e+01 false
      (:OnSuccess
        (CallFunction|AttackPlayerMelee))
      (:OnFail
        (CallFunction|FollowPlayer)))))

(event Custom|ReactToHit
  ;[0.5359 0.9301 1] Receiving damage
  (Animation|Montage|PlayMontage (Variables|Character|GetMesh) "/Game/_Main/ZombieResources/Animations/Zombie_Reaction_Hit_mixamo_com_Montage.Zombie_Reaction_Hit_mixamo_com_Montage"))

(event Custom|DeathEvent
  ;[1 0.612 0.5822] Death
  (Utilities|FlowControl|Sequence
    (:then_0
      (Variables|Default|SetisDead? true)
      (Class|BPIGameplayFramework|ZombieKilled(Message) (Game|GetGameMode)))
    (:then_1
      (Utilities|LeaveAttackingState
        (:Out
          (Utilities|DisableAllMovement)
          (Utilities|DisableAllCollisions))))
    (:then_2
      (Animation|Montage|PlayMontage (Variables|Character|GetMesh) (.OutItem (Utilities|Array|Random (Variables|Default|GetdeathMontages)))) ; Play one on the death montages
    )
    (:then_3
      ;;[1 0.4121 0.4819] Wait and destroy self
      (Utilities|FlowControl|Delay 1e+01)
      (Actor|DestroyActor))))

(event EventBeginPlay
  ;[0.4037 1 0.8073] At spawn (BeginPlay)
  (Utilities|FlowControl|Sequence
    (:then_0
      (Variables|/Script/Engine.CharacterMovementComponent|SetMaxWalkSpeed (Variables|Character|GetCharacterMovement) (Variables|Movement|GetWalkingSpeed)))
    (:then_1
      (if (Variables|Movement|GetisFollowingPlayer?)
        (CallFunction|FollowPlayer)))
    (:then_2
      ;;[0.4253 1 0.5549 0.38] Deviate ranged attack reload time
      (Variables|Combat|SetRangedAttackReloadTime (+ (Variables|Combat|GetRangedAttackReloadTime) (Math|Random|RandomFloatinRange (* (Variables|Combat|GetRangedAttackReloadTimeDeviation) -1.0) (Variables|Combat|GetRangedAttackReloadTimeDeviation))))
      (Utilities|StartRangedAttackTimer 3.0 2.0))))

(event Game|Damage|EventPointDamage
  (params (Damage :type Float%20%28single-precision%29) (DamageType :type Damage%20Type%20Object%20Reference) (HitLocation :type Vector :default "0, 0, 0") (HitNormal :type Vector :default "0, 0, 0") (HitComponent :type Primitive%20Component%20Object%20Reference) (BoneName :type Name :default "None") (ShotFromDirection :type Vector :default "0, 0, 0") (InstigatedBy :type Controller%20Object%20Reference) (DamageCauser :type Actor%20Object%20Reference) (HitInfo :type Hit%20Result%20Structure%20%28by%20ref%29))
  ;[0.5359 0.9301 1] Receiving damage
  (if (not (Variables|Default|GetisDead?))
    (CallFunction|Outrage)
    (bind _output_get (Variables|HP&Damage|SetHealth (- (Variables|HP&Damage|GetHealth) (* Damage (CallFunction|GetDamageModifierforPhysSurface (Variables|/Script/PhysicsCore.PhysicalMaterial|GetSurfaceType (.PhysMat (Collision|BreakHitResult HitInfo))))))))
    (if (> _output_get 0.0)
      (CallFunction|ReacttoHit)
      (else
        (CallFunction|DeathEvent)))))

(event Custom|AttackPlayerRanged
  (bind _returnvalue (Game|GetInstigator))
  (bind _mesh (Variables|Character|GetMesh))
  (bind _returnvalue_2 (Transformation|GetSocketTransform _mesh "BallProjectileSocket" "RTS_World"))
  ;[1 0.8593 0.3811] Throw a projectile
  (Variables|Combat|SetisAttacking? true)
  (Animation|Montage|PlayMontage (Variables|Character|GetMesh) "/Game/_Main/ZombieResources/Animations/zombie_attack_throw_Montage.zombie_attack_throw_Montage" 0.75
    (:then
      (Pawn|Components|CharacterMovement|DisableMovement (Variables|Character|GetCharacterMovement)))
    (:OnCompleted
      (Utilities|LeaveAttackingState :!label _label
        (:Out
          (CallFunction|FollowPlayer))))
    (:OnInterrupted
      (Utilities|StartRangedAttackTimer 0.0 0.0
        (:Out
          (goto _label))))
    (:OnNotifyBegin
      (Audio|PlaySoundatLocation 0 (Transformation|GetActorLocation) "0, 0, 0" 1.0 1.0 0.0 "/Game/MilitaryWeapDark/Sound/Attenuation/WeaponShot_att.WeaponShot_att" 0 self 0) ; Play zombie's projectile throwing SFX
      (Game|SpawnActorfromClass "/Game/_Main/Blueprints/Enemies/BP_ZombieProjectile.BP_ZombieProjectile_C" (Math|Transform|MakeTransform (.location _returnvalue_2) (Math|Rotator|FindLookatRotation (.location _returnvalue_2) (+ (Transformation|GetActorLocation (Game|Player|GetPlayerPawn 0)) "0,0,50.000000")) "1.000000,1.000000,1.000000") "AlwaysSpawn" _returnvalue _returnvalue)
      (Utilities|StartRangedAttackTimer 0.0 0.0))))

(event Custom|TryRangedAttack
  ;[1 1 1] Check if a ranged attack is possible
  (if (Math|Boolean|ANDBoolean (Variables|Default|GetisActive?) (not (Variables|Default|GetisDead?)) (not (Variables|Combat|GetisAttacking?)) (CallFunction|CanRangeAttackPlayer))
    (CallFunction|AttackPlayerRanged)
    (else
      (Utilities|StartRangedAttackTimer 0.0 0.0))))

(event Custom|AttackPlayerMelee
  ;[0.5052 0.1526 0.1546] Attack Player (melee)
  (Variables|Combat|SetisAttacking? true)
  (Animation|Montage|PlayMontage (Variables|Character|GetMesh) "/Game/_Main/ZombieResources/Animations/zombie_attack_Montage.zombie_attack_Montage" 1.35
    (:OnCompleted
      (Utilities|LeaveAttackingState :!label _label
        (:Out
          (CallFunction|FollowPlayer))))
    (:OnInterrupted
      (goto _label))
    (:OnNotifyBegin
      (Audio|PlaySoundatLocation 0 (Transformation|GetActorLocation) "0, 0, 0" 1.0 1.0 0.0 "/Game/MilitaryWeapDark/Sound/Attenuation/WeaponShot_att.WeaponShot_att" 0 self 0)
      ;;[1 1 1] Overlap area with a sphere, get overlapped actors (players)
      (bind (_outactors _returnvalue) (Collision|SphereOverlapActors (Transformation|GetWorldLocation (Variables|Default|GetHitboxSpawnArrow)) 5e+01 (Utilities|Array|MakeArray "ObjectTypeQuery3") "/Game/_Main/Blueprints/BP_FPPlayer.BP_FPPlayer_C" (Utilities|Array|MakeArray self)))
      (if _returnvalue
        ;;[1 1 1] Dealing damage
        (for _array_element _outactors
          (Game|Damage|ApplyDamage _array_element (Variables|Combat|GetBaseMeleeDamage) (Pawn|GetController) self "/Script/Engine.DamageType")
          (Utilities|LeaveAttackingState))))))

(fn ConstructionScript)

(fn GetDamageModifierforPhysSurface
  (params (Surface%20Type :type EPhysicalSurface%20Enum :default "SurfaceType_Default"))
  (switch Utilities|FlowControl|Switch|SwitchonEPhysicalSurface Surface%20Type
    (:SurfaceType_Default
      _)
    (:SurfaceType1
      (return (Variables|HP&Damage|GetDmgMod_Head)))
    (:SurfaceType2
      _)
    (:SurfaceType3
      (return (Variables|HP&Damage|GetDmgMod_Limbs))))
  (return (Variables|HP&Damage|GetDmgMod_Body)))

(fn CanRangeAttackPlayer
  (bind (_outhit _returnvalue) (Collision|LineTraceByChannel (+ (Transformation|GetActorLocation) "0,0,80.000000") (+ (Transformation|GetActorLocation (Game|Player|GetPlayerPawn 0)) "0,0,50.000000") "TraceTypeQuery2" false 0 "None" true "(R=0.133474,G=0.860073,B=1.000000,A=1.000000)" "(R=0.567708,G=0.019907,B=0.426765,A=1.000000)"))
  (return (and _returnvalue (Actor|ActorHasTag (.HitActor (Collision|BreakHitResult _outhit)) "Player"))))

(fn Outrage
  (Utilities|FlowControl|Sequence
    (:then_0
      ;[1 1 1] Rush at player
      (Variables|Movement|SetisRunningAtPlayer? true)
      (Variables|/Script/Engine.CharacterMovementComponent|SetMaxWalkSpeed (Variables|Character|GetCharacterMovement) (Variables|Movement|GetRunningSpeed)))))