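; Zombie spawner actor that periodically spawns enemies within a radius, starting on BeginPlay if CanSpawn is set.
; Start and stop events toggle CanSpawn and a looping timer intended to drive SpawnZombie.
; Each spawn takes its class from GetRandomEnemyClass and a random navigable X/Y with a fixed Z, then notifies the GameMode.
; The construction script sizes the SpawningArea sphere to the spawn radius.
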(event EventBeginPlay
  ;[0.4034 0.8797 1] BeginPlay
  (Utilities|FlowControl|Sequence
    (:then_1
      (if (Variables|Default|GetcanSpawn?)
        (CallFunction|StartZombieSpawning)))))

(event EventSpawnZombie
  ;[0.3979 1 0.4708] SpawnZombie event
  (if (Variables|Default|GetcanSpawn?)
    (bind _zombieinstance (Utilities|SpawnZombieinRadius))
    (Class|BPIGameplayFramework|ZombieSpawned(Message) (Game|GetGameMode) _zombieinstance)))

(event EventStartZombieSpawning
  ;[1 0.6963 0.7262] Start Zombie Spawning
  (Variables|Default|SetcanSpawn? true)
  (Utilities|StartSpawningTimer))

(event EventStopZombieSpawning
  ;[0.535 0.8791 1] Stop zombie spawning
  (Variables|Default|SetcanSpawn? false)
  (Utilities|Time|ClearandInvalidateTimerbyHandle (Variables|Default|GetZombieSpawnerTimer)))

(fn ConstructionScript
  (Components|Sphere|SetSphereRadius (Variables|Default|GetSpawningArea) (Variables|Default|GetSpawnAreaRadius) true))