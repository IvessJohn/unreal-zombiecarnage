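; FL_Utility is a Blueprint function library of helpers that switch the first local player's input mode and mouse cursor between gameplay and menus.
; DisableMenuMode hides the cursor and sets game-only input, while EnableMenuMode shows it and sets UI-only input without locking the mouse.
; SwitchInputToGameAndUI shows the cursor and allows combined game and UI input, keeping the cursor visible during capture.
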(fn DisableMenuMode
  (bind _returnvalue (Game|GetPlayerController 0))
  (Variables|/Script/Engine.PlayerController|SetbShowMouseCursor _returnvalue false)
  (Input|SetInputModeGameOnly _returnvalue))

(fn EnableMenuMode
  (bind _returnvalue (Game|GetPlayerController 0))
  (Variables|/Script/Engine.PlayerController|SetbShowMouseCursor _returnvalue true)
  (Input|SetInputModeUIOnly _returnvalue 0 "DoNotLock"))

(fn SwitchInputtoGameandUI
  (bind _returnvalue (Game|GetPlayerController 0))
  (Variables|/Script/Engine.PlayerController|SetbShowMouseCursor _returnvalue true)
  (Input|SetInputModeGameandUI _returnvalue 0 "DoNotLock" false))