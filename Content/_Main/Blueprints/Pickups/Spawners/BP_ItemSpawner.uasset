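; BP_ItemSpawner is a pickup spawner that places a random item from its ItemKinds list.
; On BeginPlay it removes its showcase mesh and spawns immediately, as the delayed first-spawn branch is bypassed by a hard-coded condition.
; The item is created by setting a ChildActor class, then cast to BP_PickupItem to bind its destruction.
; When that item is destroyed, the spawner either destroys itself (SpawnOnce) or respawns after SpawnCooldown.
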(event Custom|SpawnItem
  (bind _childactor (Variables|Default|GetChildActor))
  ;[0.1292 1 0.4669] Spawn item
  (ChildActorComponent|SetChildActorClass _childactor (.OutItem (Utilities|Array|Random (Variables|Default|GetitemKinds))))
  (bind _asbp_pickup_item (Utilities|Casting|CastToBP_PickupItem (Variables|/Script/Engine.ChildActorComponent|GetChildActor _childactor)))
  (bind _output_get (Variables|Default|SetCurrentItem _asbp_pickup_item))
  (Game|BindEventtoOnDestroyed _output_get (delegate Custom|OnSpawnedItemDestroyed)))

(event Custom|OnSpawnedItemDestroyed
  (params (DestroyedActor :type Actor%20Object%20Reference))
  ;[0.3926 1 0.9402] On current item destroyed (picked up)
  (if (Variables|Default|GetSpawnOnce)
    (Actor|DestroyActor)
    (else
      (Utilities|Time|SetTimerbyEvent (delegate Custom|SpawnItem) (Variables|Default|GetSpawnCooldown)))))

(event EventBeginPlay
  ;[1 0.8769 0.5359] BeginPlay
  (Utilities|FlowControl|Sequence
    (:then_0
      (Components|DestroyComponent (Variables|Default|GetShowcaseMesh)))
    (:then_1
      (if true
        (CallFunction|SpawnItem)
        (else
          (Utilities|Time|SetTimerbyEvent (delegate Custom|SpawnItem) (Variables|Default|GetSpawnCooldown)))))))

(fn ConstructionScript)