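; Player State for the FPS player that tracks clip and reserve ammo for each weapon type in the AmmoData map.
; BI_ interface events consume, set, add and reload ammo, changing only weapon types already in the map.
; Reload fills the clip from the reserve, capped at clip size, and returns unspent rounds to the reserve.
; Query functions report reload eligibility, clip ammo availability and the equipped weapon's ammo data.
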(event EventBIConsumeClipAmmo
  (params (weaponType :type EWeaponType%20Enum :default "NewEnumerator2"))
  (bind _ammodata (Variables|Default|GetAmmoData))
  (bind (_value _returnvalue) (Utilities|Map|Find _ammodata weaponType))
  (bind (_currentammo _totalammoleft) (Utilities|Struct|BreakAmmoDataStruct _value))
  ;[1 0.4791 0.489] Consume ammo from clip
  (if _returnvalue
    (bind _result (Math|Integer|DecrementInt _currentammo)
      (:%20%20
        (CallFunction|BISetAmmoData weaponType (Utilities|Struct|MakeAmmoDataStruct _result _totalammoleft))))))

(event EventBISetAmmoData
  (params (weaponType :type EWeaponType%20Enum :default "NewEnumerator2") (ammoData :type Ammo%20Data%20Struct%20Structure))
  (bind _ammodata (Variables|Default|GetAmmoData))
  ;[0.9909 1 0.6084] Set ammo data
  (if (.ReturnValue (Utilities|Map|Find _ammodata weaponType))
    (Utilities|Map|Add _ammodata weaponType (Utilities|Struct|MakeAmmoDataStruct (.currentammo ammoData) (.totalammoleft ammoData)))))

(event EventBIAddAmmo
  (params (weaponType :type EWeaponType%20Enum :default "NewEnumerator2") (addedAmount :type Integer))
  (bind _ammodata (Variables|Default|GetAmmoData))
  (bind (_value _returnvalue) (Utilities|Map|Find _ammodata weaponType))
  (bind (_currentammo _totalammoleft) (Utilities|Struct|BreakAmmoDataStruct _value))
  ;[1 0.8945 0.4091] Add total ammo
  (if _returnvalue
    (Utilities|Map|Add _ammodata weaponType (Utilities|Struct|MakeAmmoDataStruct _currentammo (+ _totalammoleft addedAmount)))))

(event EventBIReloadClip
  (params (weaponType :type EWeaponType%20Enum :default "NewEnumerator2") (clipSize :type Integer))
  (bind _ammodata (Variables|Default|GetAmmoData))
  (bind (_value _returnvalue) (Utilities|Map|Find _ammodata weaponType))
  (bind (_currentammo _totalammoleft) (Utilities|Struct|BreakAmmoDataStruct _value))
  (bind _returnvalue_2 (Math|Integer|Min(Integer) clipSize _totalammoleft))
  ;[0.6151 0.492 1] Reload clip
  (if _returnvalue
    (Variables|Default|SetTempAmmo _currentammo)
    (CallFunction|BISetAmmoData weaponType (Utilities|Struct|MakeAmmoDataStruct _returnvalue_2 (Math|Integer|Max(Integer) 0 (- (+ (Variables|Default|GetTempAmmo) _totalammoleft) _returnvalue_2))))))

(fn ConstructionScript)

(fn PrintAmmoDataforWeapon
  (params (weaponType :type EWeaponType%20Enum :default "NewEnumerator2"))
  (bind _ammodata (Variables|Default|GetAmmoData))
  (bind _value (Utilities|Map|Find _ammodata weaponType))
  (Development|PrintString (Utilities|String|Append "Current ammo: " (Utilities|String|ToString(Integer) (.currentammo _value)) " Total Ammo: " (Utilities|String|ToString(Integer) (.totalammoleft _value)))))

(fn BICanReload
  (params (weaponType :type EWeaponType%20Enum :default "NewEnumerator2") (clipSize :type Integer))
  (bind _ammodata (Variables|Default|GetAmmoData))
  (bind (_value _returnvalue) (Utilities|Map|Find _ammodata weaponType))
  (bind (_currentammo _totalammoleft) (Utilities|Struct|BreakAmmoDataStruct _value))
  (if _returnvalue
    (return (and (< _currentammo clipSize) (> _totalammoleft 0)))
    (else
      (return false))))

(fn BIGetCurrentWeaponAmmoData
  (bind _ammodata (Variables|Default|GetAmmoData))
  (bind _equippedweaponref (Variables|Default|GetEquippedWeaponRef))
  (bind _weapontype (Variables|/Game/_Main/Blueprints/Weapons/BP_WeaponParent.BP_WeaponParent_C|GetWeaponType _equippedweaponref))
  (bind (_value _returnvalue) (Utilities|Map|Find _ammodata _weapontype))
  (bind (_currentammo _totalammoleft) (Utilities|Struct|BreakAmmoDataStruct _value))
  (Utilities|IsValid _equippedweaponref
    (:Is%20Valid
      (if _returnvalue
        (return _currentammo (Variables|/Game/_Main/Blueprints/Weapons/BP_WeaponParent.BP_WeaponParent_C|GetClipSize (Variables|Default|GetEquippedWeaponRef)) _totalammoleft)))))

(fn BIHasAmmoinClip
  (params (weaponType :type EWeaponType%20Enum :default "NewEnumerator2"))
  (bind _ammodata (Variables|Default|GetAmmoData))
  (bind (_value _returnvalue) (Utilities|Map|Find _ammodata weaponType))
  (if _returnvalue
    (return (> (.CurrentAmmo (Utilities|Struct|BreakAmmoDataStruct _value)) 0))
    (else
      (return false))))