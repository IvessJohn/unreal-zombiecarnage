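; Player controller for the first-person player that owns the game's UI and pause flow.
; On possess it caches the player and creates the HUD and fade-out screen, then forwards reload and weapon-swap input to the player.
; Health, wave and intermission events are relayed to the HUD as messages.
; Level end blocks pausing, swaps the HUD for an end screen that shows complete or failed, and disables player actions.
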(event EventFinishedReloading
  ;[0.1146 0.1146 0.1146 1 42] Weapons
  ;;[1 0.4708 0.9454] Reload Action
  (CallFunction|HideReloadingText))

(event EventHideReloadingText
  ;[0.1146 0.1146 0.1146 1 42] Weapons
  ;;[1 0.4708 0.9454] Reload Action
  (Default|HideReloading (Variables|Default|GetGameHUD)))

(event EventPossess
  (params (PossessedPawn :type Pawn%20Object%20Reference))
  (bind _self self)
  ;[0.609 0.7279 1] On Possess - save player reference, set up UI
  (Utilities|FlowControl|Sequence
    (:then_0
      (bind _asbp_fpplayer (Utilities|Casting|CastToBP_FPPlayer PossessedPawn))
      (Variables|Default|SetPlayerRef _asbp_fpplayer))
    (:then_1
      ;;[1 1 1] Set input mode to Game Only
      (CallFunction|DisableMenuMode))
    (:then_2
      ;;[0.9531 0.4052 0.1838] Set up UI
      (Utilities|FlowControl|Sequence
        (:then_0
          (bind _returnvalue (UserInterface|CreateWidget "/Game/_Main/UI/W_GameHUD.W_GameHUD_C" _self))
          (bind _output_get (Variables|Default|SetGameHUD _returnvalue))
          (UserInterface|Viewport|AddtoViewport _output_get 0))
        (:then_1
          (bind _returnvalue_2 (UserInterface|CreateWidget "/Game/_Main/UI/W_FadeOutScreen.W_FadeOutScreen_C" _self))
          (UserInterface|Viewport|AddtoViewport _returnvalue_2 0))))))

(event EventShowBloodyScreen
  ;[0.7677 1 0.3355 1 40] Low health events
  ;;[1 0.3603 0.3105] Show Bloody Screen on player's injury
  (Class|BPIatLowHealth|ShowBloodyScreen(Message) (Variables|Default|GetGameHUD)))

(event EventNoLongerLowHealth
  ;[0.7677 1 0.3355 1 40] Low health events
  ;;[0.3575 0.8183 1] Show/Hide low health redness
  (Class|BPIatLowHealth|NoLongerLowHealth(Message) (Variables|Default|GetGameHUD)))

(event EventReachedLowHealth
  ;[0.7677 1 0.3355 1 40] Low health events
  ;;[0.3575 0.8183 1] Show/Hide low health redness
  (Class|BPIatLowHealth|ReachedLowHealth(Message) (Variables|Default|GetGameHUD)))

(event Input|ActionEvents|InputActionReload
  (params (Key :type Key%20Structure :default "None"))
  ;[0.1146 0.1146 0.1146 1 42] Weapons
  ;;[1 0.4708 0.9454] Reload Action
  (:Pressed
    (bind _canreload (Default|Reload (Variables|Default|GetPlayerRef)))
    (if _canreload
      (Default|ShowReloading (Variables|Default|GetGameHUD)))))

(event Input|ActionEvents|InputActionPauseGame
  (params (Key :type Key%20Structure :default "None"))
  ;[1 0.6475 0.9756] Pause Game
)

(event Input|ActionEvents|InputActionHotkey_Primary
  (params (Key :type Key%20Structure :default "None"))
  (bind _playerref (Variables|Default|GetPlayerRef))
  ;[0.1146 0.1146 0.1146 1 42] Weapons
  ;;[0.5336 0.8157 1] Weapon switching
  (:Pressed
    (Default|EquipGun _playerref (Variables|/Game/_Main/Blueprints/Player/BP_FPPlayer.BP_FPPlayer_C|GetPrimaryWeaponClass _playerref))))

(event Input|ActionEvents|InputActionHotkey_Secondary
  (params (Key :type Key%20Structure :default "None"))
  (bind _playerref (Variables|Default|GetPlayerRef))
  ;[0.1146 0.1146 0.1146 1 42] Weapons
  ;;[0.5336 0.8157 1] Weapon switching
  (:Pressed
    (Default|EquipGun _playerref (Variables|/Game/_Main/Blueprints/Player/BP_FPPlayer.BP_FPPlayer_C|GetSecondaryWeaponClass _playerref))))

(event Input|ActionEvents|InputActionSwapWeapons
  (params (Key :type Key%20Structure :default "None"))
  ;[0.1146 0.1146 0.1146 1 42] Weapons
  ;;[0.5336 0.8157 1] Weapon switching
  (:Pressed
    (Default|SwitchWeapons (Variables|Default|GetPlayerRef))))

(event Input|KeyboardEvents|P
  (params (Key :type Key%20Structure :default "None"))
  ;[1 0.6475 0.9756] Pause Game
  ;;[1 0.07146 0.1212] TODO: Replace these with InputAction PauseGame
  (:Pressed
    (if (Variables|Default|GetcanTogglePause?)
      (CallFunction|TogglePause))))

(event Input|KeyboardEvents|Escape
  (params (Key :type Key%20Structure :default "None"))
  ;[1 0.6475 0.9756] Pause Game
  ;;[1 0.07146 0.1212] TODO: Replace these with InputAction PauseGame
  (:Pressed
    (if (Variables|Default|GetcanTogglePause?)
      (CallFunction|TogglePause))))

(event EventLevelEnd
  (bind _pausemenuui (Variables|Default|GetPauseMenuUI))
  ;[0.3541 0.5931 1 1 40] Level end: end, complete, fail
  ;;[0.954 0.6634 1] Level End
  (Utilities|FlowControl|Sequence
    (:then_0
      (Variables|Default|SetcanTogglePause? false)
      (CallFunction|UnpauseGame))
    (:then_1
      ;;;[1 0.8022 0.669 1 16] Remove UI
      (Widget|RemovefromParent (Variables|Default|GetGameHUD))
      (Utilities|IsValid _pausemenuui
        (:Is%20Valid
          (Widget|RemovefromParent _pausemenuui))))
    (:then_2
      ;;;[0.7186 1 0.8171 1 16] Add level end screen
      (CallFunction|EnableMenuMode)
      (bind _returnvalue (UserInterface|CreateWidget "/Game/_Main/UI/W_LevelEndScreen.W_LevelEndScreen_C" self))
      (bind _output_get (Variables|Default|SetLevelEndScreen _returnvalue))
      (UserInterface|Viewport|AddtoViewport _output_get 0))
    (:then_3
      (Default|DisableMovementandActions (Variables|Default|GetPlayerRef)))))

(event EventWaveEnded
  ;[1 0.739 0.2663 1 40] Wave-related
  ;;[1 1 1] Wave ended
  (Class|BPIGameplayFramework|WaveEnded(Message) (Variables|Default|GetGameHUD)))

(event EventWaveStarted
  ;[1 0.739 0.2663 1 40] Wave-related
  ;;[1 1 1] Wave started
  (Class|BPIGameplayFramework|WaveStarted(Message) (Variables|Default|GetGameHUD)))

(event EventIntermissionStarted
  ;[1 0.739 0.2663 1 40] Wave-related
  ;;[1 1 1] Intermission started
  (Class|BPIGameplayFramework|IntermissionStarted(Message) (Variables|Default|GetGameHUD)))

(event EventLevelComplete
  ;[0.3541 0.5931 1 1 40] Level end: end, complete, fail
  ;;[0.3091 1 0.3049] Level Complete
  (Class|BPIGameplayFramework|LevelComplete(Message) (Variables|Default|GetLevelEndScreen)))

(event EventLevelFailed
  ;[0.3541 0.5931 1 1 40] Level end: end, complete, fail
  ;;[1 0.5501 0.59] Level failed
  (Class|BPIGameplayFramework|LevelFailed(Message) (Variables|Default|GetLevelEndScreen)))

(fn ConstructionScript)

(fn ShowPauseMenu
  (Utilities|FlowControl|Sequence
    (:then_0
      (Utilities|IsValid (Variables|Default|GetPauseMenuUI)
        (:Is%20Not%20Valid
          ;[1 1 1] Invalid -> Create widget
          (bind _returnvalue (UserInterface|CreateWidget "/Game/_Main/UI/W_PauseMenu.W_PauseMenu_C" self))
          (bind _output_get (Variables|Default|SetPauseMenuUI _returnvalue))
          (UserInterface|Viewport|AddtoViewport _output_get 0))))
    (:then_1
      ;[1 1 1] Valid -> Set visibility to Visible
      (Default|Show (Variables|Default|GetPauseMenuUI)))))

(fn TogglePause
  (if (not (Game|IsGamePaused))
    (CallFunction|PauseGame)
    (else
      (CallFunction|UnpauseGame))))

(fn PauseGame
  (CallFunction|ShowPauseMenu)
  (Game|SetGamePaused true))

(fn UnpauseGame
  (if (Game|IsGamePaused)
    (Default|ResumeGame (Variables|Default|GetPauseMenuUI))))